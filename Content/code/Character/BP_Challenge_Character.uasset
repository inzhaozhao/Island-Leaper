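; BP_Challenge_Character is the player character for a challenge mode where dropping below a fixed height means death and respawn.
; Enhanced Input mappings added on BeginPlay drive camera-relative movement, look and jump.
; Tick checks the height and calls Dead, which enables mesh ragdoll physics, disables spring arm collision and stops movement.
; After a short delay, Dead destroys the actor and calls Rebirth on BP_ChanllengeMode.
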(event Custom|Dead
  (Physics|SetSimulatePhysics (Variables|Character|GetMesh) true)
  (Variables|/Script/Engine.SpringArmComponent|SetbDoCollisionTest (Variables|Default|GetSpringArm) false)
  (Pawn|Components|CharacterMovement|SetMovementMode (Variables|Character|GetCharacterMovement) "MOVE_None" 0)
  (Utilities|FlowControl|Delay 2.0)
  (Actor|DestroyActor)
  (bind _asbp_chanllenge_mode (Utilities|Casting|CastToBP_ChanllengeMode (Game|GetGameMode)))
  (Default|Rebirth _asbp_chanllenge_mode))

(event Input|EnhancedActionEvents|EnhancedInputActionIA_Move
  (params (ActionValue :type Vector%202D%20Structure) (ElapsedSeconds :type Float%20%28double-precision%29) (TriggeredSeconds :type Float%20%28double-precision%29) (InputAction :type Input%20Action%20Object%20Reference :default "/Game/code/Character/Input/IA_Move.IA_Move"))
  (bind (_x _y) (Math|Vector2D|BreakVector2D ActionValue))
  (bind _camera (Variables|Default|GetCamera))
  (Pawn|Input|AddMovementInput (Math|Vector|GetForwardVector _camera) _x false)
  (Pawn|Input|AddMovementInput (Math|Vector|GetRightVector _camera) _y false))

(event Input|EnhancedActionEvents|EnhancedInputActionIA_Iook
  (params (ActionValue :type Vector%202D%20Structure) (ElapsedSeconds :type Float%20%28double-precision%29) (TriggeredSeconds :type Float%20%28double-precision%29) (InputAction :type Input%20Action%20Object%20Reference :default "/Game/code/Character/Input/IA_Iook.IA_Iook"))
  (bind (_x _y) (Math|Vector2D|BreakVector2D ActionValue))
  (Pawn|Input|AddControllerYawInput _x)
  (Pawn|Input|AddControllerPitchInput _y))

(event Input|EnhancedActionEvents|EnhancedInputActionIA_Jump
  (params (ActionValue :type Boolean) (ElapsedSeconds :type Float%20%28double-precision%29) (TriggeredSeconds :type Float%20%28double-precision%29) (InputAction :type Input%20Action%20Object%20Reference :default "/Game/code/Character/Input/IA_Jump.IA_Jump"))
  (:Started
    (Character|Jump)))

(event EventBeginPlay
  (Input|AddMappingContext (PlayerController|LocalPlayerSubsystems|GetEnhancedInputLocalPlayerSubsystem (Game|GetPlayerController 0)) "/Game/code/Character/Input/IMC_Challenge.IMC_Challenge" 0 "(bIgnoreAllPressedKeysUntilRelease=True,bForceImmediately=False,bNotifyUserSettings=False)"))

(event EventTick
  (params (DeltaSeconds :type Float%20%28single-precision%29))
  (if (<= (.z (Transformation|GetActorLocation)) 452.0)
    (CallFunction|Dead)))

(fn ConstructionScript)