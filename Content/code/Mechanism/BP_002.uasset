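; BP_002 is a mechanism Blueprint that moves two wooden pole meshes vertically in a counter-motion.
; On BeginPlay it caches both relative locations, with each variable taking the other pole's position, then plays a timeline.
; Each update raises pole 06 by the track value and pole 08 by that value's absolute difference from 150, each based on the other pole's starting position.
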(event EventBeginPlay
  (Variables|Default|Set06Location (Variables|/Script/Engine.SceneComponent|GetRelativeLocation (Variables|Default|GetSM_WoodenPole_08)))
  (Variables|Default|Set08Location (Variables|/Script/Engine.SceneComponent|GetRelativeLocation (Variables|Default|GetSM_WoodenPole_06)))
  (bind _新建轨道_0 (Timeline|时间轴 Play)
    (:Update
      (Transformation|SetRelativeLocation (Variables|Default|GetSM_WoodenPole_06) (Math|Vector|MakeVector (.x (Variables|Default|Get06Location)) (.y (Variables|Default|Get06Location)) (+ (.z (Variables|Default|Get06Location)) _新建轨道_0)) false false)
      (Transformation|SetRelativeLocation (Variables|Default|GetSM_WoodenPole_08) (Math|Vector|MakeVector (.x (Variables|Default|Get08Location)) (.y (Variables|Default|Get08Location)) (+ (.z (Variables|Default|Get08Location)) (Math|Float|Absolute(Float) (- _新建轨道_0 1.5e+02)))) false false))))

(fn ConstructionScript)