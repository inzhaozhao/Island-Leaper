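; BP_003 is a spinning obstacle that either kills or launches a challenge character touching its Capsule.
; Body rotates a fixed step every Tick, without delta-time scaling.
; On overlap, the Death flag selects between calling Dead, or calling Jump and adding a strong impulse along the Arrow's forward vector.
; The construction script shows the Thorn when Death is set and toggles the base mesh from the Base flag.
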(event OnComponentBeginOverlap(Capsule)
  (params (OverlappedComponent :type Primitive%20Component%20Object%20Reference) (OtherActor :type Actor%20Object%20Reference) (OtherComp :type Primitive%20Component%20Object%20Reference) (OtherBodyIndex :type Integer) (bFromSweep :type Boolean) (SweepResult :type Hit%20Result%20Structure%20%28by%20ref%29))
  (bind _asbp_challenge_character (Utilities|Casting|CastToBP_Challenge_Character OtherActor))
  (if (Variables|Default|GetDeath)
    (Default|Dead _asbp_challenge_character)
    (else
      (Character|Jump _asbp_challenge_character)
      (Physics|AddImpulse (Variables|/Script/Engine.Character|GetCharacterMovement _asbp_challenge_character) (* (Math|Vector|GetForwardVector (Variables|Default|GetArrow)) 20000) false))))

(event EventTick
  (params (DeltaSeconds :type Float%20%28single-precision%29))
  (Transformation|AddRelativeRotation (Variables|Default|GetBody) "0.000000,5.000000,0.000000" false false))

(fn ConstructionScript
  (if (Variables|Default|GetDeath)
    (Rendering|SetVisibility (Variables|Default|GetThorn) true false)
    (else
      (Rendering|SetVisibility (Variables|Default|GetThorn) false false)))
  (if (Variables|Default|GetBase)
    (Rendering|SetVisibility (Variables|Default|GetBase1) true false)
    (else
      (Rendering|SetVisibility (Variables|Default|GetBase1) false false))))